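; Test Blueprint that demonstrates fuzzy string matching, such as correcting typos in color names against a valid color list.
; BeginPlay fills KnownStrings with valid, near-miss, bad and random inputs, then runs each through FindClosestString against ValidColors, leaving results unused.
; FindClosestString returns the best matches by cosine similarity over character bigrams, possibly several.
; It also runs FilterStrings on any digits in the input, but that result is unused.
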(event EventBeginPlay
  (Utilities|FlowControl|Sequence
    (:then_0
      ;[0.08854 0.006029 0] Simulate User Input
      ; via 'Known Strings' which contains strings we want to test
      ; Appends the example you wish to include
      (Utilities|Array|AppendArray (Variables|Default|GetknownStrings) (Variables|Default|GetvalidColors)) ; Colors that will match
      (Utilities|Array|AppendArray (Variables|Default|GetknownStrings) (Variables|Default|GetcloseColors)) ; The Use Case, typos in colors
      (Utilities|Array|AppendArray (Variables|Default|GetknownStrings) (Variables|Default|GetbadColors)) ; Isnt expected to match anything, but might
      (Utilities|Array|AppendArray (Variables|Default|GetknownStrings) (Variables|Default|GetrandomInput)) ; Isnt expected to match anything, but might
    )
    (:then_1
      (for _array_element (Variables|Default|GetknownStrings)
        (bind _closestitemsout (CallFunction|FindClosestString _array_element (Variables|Default|GetvalidColors))) ; Closest Items Out should be one element, however it could match on multiple. Grab first element in the array or filter further.\nLogs are disabled by default. To enable them there is a boolean inside this function.
      ))))

(fn ConstructionScript)

(fn FindClosestString
  (params (inputString :type String) (validStringList :type Array%20of%20Strings))
  ;[0.1562 0.07858 0 1 10] This function extracts all numeric characters from a given string and concatenates them into a new string, effectively filtering out all non-numeric characters.
  ;
  ; Inputs:
  ; String (String): The input string from which numeric characters are to be extracted.
  ;
  ; Output:
  ; Numeric Part (String): A string composed of only the numeric characters extracted from the input string.
  ;
  ; Workflow:
  ; The function receives a string as input.
  ; It breaks the string into individual characters.
  ; Each character is then checked to determine if it is numeric.
  ; Numeric characters are concatenated to form the 'Numeric String'.
  ; The process continues until all characters have been evaluated.
  ; The function outputs the 'Numeric String'.
  ;
  ; Use Case Example:
  ; Given the input string "abc123def45", the function will return "12345".
  ;
  ; Notes:
  ; The function only considers standard numeric characters (0-9).
  ; If the input string contains no numeric characters, an empty string is returned.
  ; This function is useful in scenarios where numeric data is embedded within non-numeric text and needs to be isolated for calculations or other numeric processing.
  (bind _numericpart (CallFunction|StringExtractNumber inputString))
  (if (Utilities|Array|IsEmpty _numericpart)
    _
    (else
      ;[0.1562 0.07858 0 1 10] This function filters an array of strings, returning a new array that only includes strings containing a specified substring. It's useful for narrowing down a list based on a search term or specific criteria.
      ;
      ; Inputs:
      ; Array of Strings (Input Array): The original array of strings to be filtered.
      ; Substring (String): The substring to search for within each string of the array.
      ;
      ; Output:
      ; Filtered Array (Output Array): An array containing only those strings from the input array that include the specified substring.
      ;
      ; Workflow:
      ; The function iterates over each string in the input array.
      ; For each string, it checks if the specified substring is present.
      ; If the substring is found, the string is added to the 'Filtered Array'.
      ; The process repeats until all strings in the input array have been evaluated.
      ; The function then outputs the 'Filtered Array'.
      ;
      ; Use Case Example:
      ; Given an array ["apple", "banana", "grape", "blueberry"] and a substring "a", the function will return ["apple", "banana", "grape"].
      ;
      ; Notes:
      ; The search is case-insensitive by default.
      ; If no substring is provided, the original array is returned.
      ; If the original array is empty, an empty array is returned.
      (CallFunction|FilterStrings validStringList _numericpart)))
  ;[0.1562 0.07858 0 1 10] Function Name: Find Closest String Cosine Ngram
  ;
  ; Description: This function evaluates the similarity between a reference string and an array of comparison strings using the cosine similarity method with n-gram analysis. By converting strings into n-gram frequency vectors, it calculates the cosine similarity to identify the string(s) in the array that are most similar to the reference string. It's designed for applications requiring semantic text analysis, such as search algorithms, data cleaning, or natural language processing tasks where the exact match is not crucial but closeness in context or meaning is.
  ;
  ; Inputs:
  ; String A (String): The reference string to compare against.
  ; String List (Array of Strings): The list of strings to be compared to String A.
  ; N (Integer): Determines the n-gram size for the analysis. Affects the granularity of the matching process.
  ; Logs Enabled (Boolean): When true, enables the logging of function operations for debugging or analytical purposes.
  ;
  ; Outputs:
  ; Closest Matches Out (Array of Strings): Outputs an array of strings that are closest to the reference string based on the cosine similarity score. This array may contain one or more strings if multiple strings share the same highest similarity score.
  ;
  ; Workflow:
  ; N-Gram Generation: Converts String A and each string in the String List into sets of n-grams based on the specified value of N.
  ; Vector Mapping: Creates frequency vectors (Vector Map A and Vector Map B) for the generated n-grams, capturing the occurrence of each n-gram within the strings.
  ; Cosine Similarity Calculation: Computes the dot product and magnitudes of the frequency vectors to calculate the cosine similarity between String A and each string in the list.
  ; Identification of Closest Matches: Determines which string(s) have the highest cosine similarity to String A and prepares them for output.
  ; Output Generation: Returns the Closest Matches Out array containing the string(s) most similar to String A, alongside the cosine similarity score for reference.
  ;
  ; Use Case Example:
  ; Suppose String A is "example", and the String List contains ["sample", "examine", "simple", "example"]. With N set to 2, the function might return ["example"] as the Closest Matches Out, indicating an exact match or the highest similarity.
  ;
  ; Notes:
  ; The choice of N significantly affects the analysis's sensitivity and specificity. Smaller values of N may capture more general similarities, while larger values highlight more specific features.
  ; Performance considerations are essential for large datasets or high values of N, as the computational complexity increases with the size of the data and the granularity of the analysis.
  ; Enabling logs can provide valuable insights into the function's internal processes and decision-making but may impact performance due to the additional overhead.
  (bind _closestmatches_out (CallFunction|FindClosestStringCosineNgram inputString validStringList 2 false))
  (return _closestmatches_out))