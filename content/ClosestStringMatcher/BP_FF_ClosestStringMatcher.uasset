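; Demo Blueprint for fuzzy string matching, testing color names, typos and random input against a list of valid colors.
; BeginPlay builds the test list and runs FindClosestString on each entry, leaving the results unused.
; FindClosestString filters candidates by any number extracted from the input, then scores them with cosine n-gram similarity on two-character segments, with logging enabled.
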(event EventBeginPlay
  (Utilities|FlowControl|Sequence
    (:then_0
      ;[0.08854 0.006029 0] Simulate User Input
      ; via 'Color List' which contains strings we want to test
      ; Appends the example you wish to include
      (Utilities|Array|AppendArray (Variables|Default|GetknownStrings) (Variables|Default|GetvalidColors)) ; Colors that will match
      (Utilities|Array|AppendArray (Variables|Default|GetknownStrings) (Variables|Default|GetbadColors)) ; Isnt expected to match anything, but might
      (Utilities|Array|AppendArray (Variables|Default|GetknownStrings) (Variables|Default|GetcloseColors)) ; The Use Case, typos in colors
      (Utilities|Array|AppendArray (Variables|Default|GetknownStrings) (Variables|Default|GetrandomInput)) ; Isnt expected to match anything, but might
    )
    (:then_1
      (for _array_element (Variables|Default|GetknownStrings)
        (bind _closestitemsout (CallFunction|FindClosestString _array_element (Variables|Default|GetvalidColors))) ; Closest Items Out should be one element, however it could match on multiple. Grab first element in the array or filter further.\nLogs are disabled by default. To enable them there is a boolean inside this function.
      ))))

(fn ConstructionScript)

(fn FindClosestString
  (params (inputString :type String) (validStringList :type Array%20of%20Strings))
  (bind _numericpart (CallFunction|StringExtractNumber inputString))
  (if (Utilities|Array|IsEmpty _numericpart)
    _
    (else
      (CallFunction|FilterStrings validStringList _numericpart) ; If theres numerics, remove non matching values from our valid list.\nThis prevents blu2 from matching on [blue, blue3] \nby only allowing the valid list to contain strings with 2
    ))
  (bind _closestmatches_out (CallFunction|FindClosestStringCosineNgram inputString validStringList 2 true)) ; String A: is your input string to search a closest match for.\nString List: The list of valid or known string values to match on\nN: Length of each segment (e.g., 3 in "cat" for 3-gram). Adjust N for finer or broader analysis granularity.\n\nClosest Matches Out: Array of results. Ideally will match with an array of 1. ['red'] However if it fails or matches on multiple this can be multiple. \nCheck length === 1 to determine if matched. Also grab first element as its the result youll want.\n\nCheck Logs Enabled to log out the results.
  (return _closestmatches_out))