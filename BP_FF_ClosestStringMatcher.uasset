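; Test actor that demonstrates fuzzy matching of typo-prone color names against a list of valid colors.
; BeginPlay merges valid, bad, near-miss and random sample inputs, then runs each through FindClosestString.
; That function filters candidates by any number found in the input, then picks the closest using bigram cosine similarity.
; The match results are not used further in the graph.
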(event EventBeginPlay
  (Utilities|FlowControl|Sequence
    (:then_0
      ;[0.08854 0.006029 0] Simulate User Input
      ; via 'Color List' which contains strings we want to test
      ; Appends the example you wish to include
      (Utilities|Array|AppendArray (Variables|Default|GetknownStrings) (Variables|Default|GetvalidColors)) ; Colors that will match
      (Utilities|Array|AppendArray (Variables|Default|GetknownStrings) (Variables|Default|GetbadColors)) ; Isnt expected to match anything, but might
      (Utilities|Array|AppendArray (Variables|Default|GetknownStrings) (Variables|Default|GetcloseColors)) ; The Use Case, typos in colors
      (Utilities|Array|AppendArray (Variables|Default|GetknownStrings) (Variables|Default|GetrandomInput)) ; Isnt expected to match anything, but might
    )
    (:then_1
      (for _array_element (Variables|Default|GetknownStrings)
        (bind _closestitemsout (CallFunction|FindClosestString _array_element (Variables|Default|GetvalidColors))) ; Closest Items Out should be one element, however it could match on multiple. Grab first element in the array or filter further.\nLogs are disabled by default. To enable them there is a boolean inside this function.
      ))))

(fn ConstructionScript)

(fn FindClosestString
  (params (inputString :type String) (validStringList :type Array%20of%20Strings))
  (bind _numericpart (CallFunction|StringExtractNumber inputString))
  (if (Utilities|Array|IsEmpty _numericpart)
    _
    (else
      (CallFunction|FilterStrings validStringList _numericpart) ; If theres numerics, remove non matching values from our valid list.
    ))
  (bind _closestmatches_out (CallFunction|FindClosestStringCosineNgram inputString validStringList 2 false))
  (return _closestmatches_out))